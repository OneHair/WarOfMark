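; Player character base Blueprint that gives the player a toggleable inventory screen.
; On BeginPlay it creates the BPW_Main widget, stores it as the inventory reference and adds it to the viewport collapsed.
; Tab drives a FlipFlop that either shows the widget with the mouse cursor and refreshes its list from the Bag variable, or hides both.
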(event `self.ReceiveBeginPlay`
  (`self.InventoryInitial`))

(event `InventoryInitial`
  (bind _returnvalue (`|CreateWidget` "/Game/Blueprint/Widget/BPW_Main.BPW_Main_C"))
  (bind _output_get (set `self.InventorySystemRef` _returnvalue))
  (`UserWidget.AddToViewport` _output_get 0)
  (`Widget.SetVisibility` _output_get "Collapsed"))

(event `Key|Tab`
  (params (Key :type "Key Structure"))
  (bind _returnvalue (`GameplayStatics.GetPlayerController` 0))
  (bind _inventorysystemref (`self.InventorySystemRef`))
  (:`Pressed`
    (`/Engine/EditorBlueprintResources/StandardMacros.IsValid` (`self.InventorySystemRef`)
      (:`Is Valid`
        (`/Engine/EditorBlueprintResources/StandardMacros.FlipFlop`
          (:`A`
            (`Widget.SetVisibility` _inventorysystemref "Visible")
            (set `PlayerController.bShowMouseCursor` true _returnvalue)
            (`/Game/Blueprint/Widget/BPW_InventoryList.UpdateList` (`/Game/Blueprint/Widget/BPW_Main.BPW_InventoryList_C_0` (`self.InventorySystemRef`)) (`self.Bag`)))
          (:`B`
            (`Widget.SetVisibility` _inventorysystemref "Collapsed")
            (set `PlayerController.bShowMouseCursor` false _returnvalue)))))))

(fn `UserConstructionScript`)